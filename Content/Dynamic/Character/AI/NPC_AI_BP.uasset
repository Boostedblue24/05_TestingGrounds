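; AI controller for guard NPCs that sets up the PatrolData blackboard and runs the GuardBehavior behavior tree on BeginPlay.
; AI perception updates write sensed actors without the "Enemy" tag to the blackboard's enemy key and clear it on lost stimulus.
; Both writes require the controlled pawn to be a BP_TestingGroundsCharacter.
; A disconnected chain would set the pawn's Aiming and Shooting from focus-actor validity, but never runs.
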(event `self.ReceiveBeginPlay`
  (bind _blackboardcomponent (`self.UseBlackboard` "/Game/Dynamic/Character/AI/PatrolData.PatrolData"))
  (`self.RunBehaviorTree` "/Game/Dynamic/Character/AI/GuardBehavior.GuardBehavior")
  (set `self.BlackboardComp` _blackboardcomponent))

(event `self.AIPerception.OnTargetPerceptionUpdated`
  (params (Actor :type "Actor Object Reference") (Stimulus :type "AIStimulus Structure"))
  (`self.UpdateBlackBoardEnemyKey` Actor Stimulus Actor))

(event `self.ReceiveTick`
  (params (DeltaSeconds :type "Float (single-precision)")))

(fn `UpdateBlackBoardEnemyKey`
  (params (self2 :type "Actor Object Reference") (AIStimulus :type "AIStimulus Structure (by ref)") (ObjectValue :type "Object Object Reference"))
  (bind _enemykey (`self.EnemyKey`))
  (bind _blackboardcomp (`self.BlackboardComp`))
  (`/Engine/EditorBlueprintResources/StandardMacros.IsValid` self2
    (:`Is Valid`
      (if (`self.ActorHasTag` self2 "Enemy")
        _
        (elif (`.bSuccessfullySensed` (break `AIStimulus` AIStimulus))
          (cast `/Game/Dynamic/Character/Behavior/BP_TestingGroundsCharacter` (`self.K2_GetPawn`))
          (`BlackboardComponent.SetValueAsObject` _blackboardcomp _enemykey ObjectValue)
          (else
            (cast `/Game/Dynamic/Character/Behavior/BP_TestingGroundsCharacter` (`self.K2_GetPawn`))
            (`BlackboardComponent.ClearValue` _blackboardcomp _enemykey)))))))

(fn `UserConstructionScript`)
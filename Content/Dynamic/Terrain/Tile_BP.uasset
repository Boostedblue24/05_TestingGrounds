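; Terrain tile for an infinite-terrain level, which scatters containers, crates, canisters, rocks and sandbags through PlaceActors and attaches them on BeginPlay.
; Its barrier starts solid red, turns green and passable when the player enters BarrierCollision, then relocks on exit as InfiniteTerrainGameMode spawns another tile.
; The tile exposes its Arrow transform as an attach location and destroys itself when the player overlaps DestroyTileCollision.
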(event `self.ReceiveBeginPlay`
  (`self.LockLevel`)
  (`self.PlaceAndAttachAllActors`))

(event `self.BarrierCollision.OnComponentBeginOverlap`
  (params (OverlappedComponent :type "PrimitiveComponent Object Reference") (OtherActor :type "Actor Object Reference") (OtherComp :type "PrimitiveComponent Object Reference") (OtherBodyIndex :type Integer) (bFromSweep :type Boolean) (SweepResult :type "HitResult Structure (by ref)"))
  (`self.IsPlayerActor` OtherActor)
  (`self.UnlockLevel`))

(event `self.BarrierCollision.OnComponentEndOverlap`
  (params (OverlappedComponent :type "PrimitiveComponent Object Reference") (OtherActor :type "Actor Object Reference") (OtherComp :type "PrimitiveComponent Object Reference") (OtherBodyIndex :type Integer))
  (`self.IsPlayerActor` OtherActor)
  (`self.LockLevel`)
  (bind _asinfinite_terrain_game_mode (cast `/Game/Dynamic/InfiniteTerrainGameMode` (`GameplayStatics.GetGameMode`)))
  (`/Game/Dynamic/InfiniteTerrainGameMode.SpawnTile` _asinfinite_terrain_game_mode))

(event `self.DestroyTileCollision.OnComponentBeginOverlap`
  (params (OverlappedComponent :type "PrimitiveComponent Object Reference") (OtherActor :type "Actor Object Reference") (OtherComp :type "PrimitiveComponent Object Reference") (OtherBodyIndex :type Integer) (bFromSweep :type Boolean) (SweepResult :type "HitResult Structure (by ref)"))
  (`self.IsPlayerActor` OtherActor)
  (`self.K2_DestroyActor`))

(fn `GetAttachLocation`
  (returns (AttachTransform :type "Transform Structure"))
  (return (`SceneComponent.K2_GetComponentToWorld` (`self.Arrow`))))

(fn `LockLevel`
  (bind _barrier (`self.Barrier`))
  (`PrimitiveComponent.SetCollisionEnabled` _barrier "QueryAndPhysics")
  (`PrimitiveComponent.SetMaterial` _barrier 0 "/Game/Dynamic/Terrain/MI_Barrier_Red.MI_Barrier_Red"))

(fn `PlaceAndAttachAllActors`
  (`self.PlaceActors` "/Game/Dynamic/Terrain/Props/Container_BP.Container_BP_C" 0 3 400.0)
  (`self.K2_AttachToActor` null "None" "KeepRelative" "KeepRelative" "KeepRelative" false)
  (`self.PlaceActors` "/Game/Dynamic/Terrain/Props/Box_BP.Box_BP_C" 1 5 100.0)
  (`self.K2_AttachToActor` null "None" "KeepRelative" "KeepRelative" "KeepRelative" false)
  (`self.PlaceActors` "/Game/Dynamic/Terrain/Props/Canister_BP.Canister_BP_C" 1 5 50.0)
  (`self.K2_AttachToActor` null "None" "KeepRelative" "KeepRelative" "KeepRelative" false)
  (`self.PlaceActors` "/Game/Dynamic/Terrain/Props/Rock01_BP.Rock01_BP_C" 1 4 150.0 1.0 5.0)
  (`self.K2_AttachToActor` null "None" "KeepRelative" "KeepRelative" "KeepRelative" false)
  (`self.PlaceActors` "/Game/Dynamic/Terrain/Props/Rock05_BP.Rock05_BP_C" 0 2 250.0 1.0 4.0)
  (`self.K2_AttachToActor` null "None" "KeepRelative" "KeepRelative" "KeepRelative" false)
  (`self.PlaceActors` "/Game/Dynamic/Terrain/Props/Rock17_BP.Rock17_BP_C" 0 3 250.0 1.0 3.0)
  (`self.K2_AttachToActor` null "None" "KeepRelative" "KeepRelative" "KeepRelative" false)
  (`self.PlaceActors` "/Game/Dynamic/Terrain/Props/Sandbags.Sandbags_C" 1 2 250.0)
  (`self.K2_AttachToActor` null "None" "KeepRelative" "KeepRelative" "KeepRelative" false))

(fn `UnlockLevel`
  (bind _barrier (`self.Barrier`))
  (`PrimitiveComponent.SetCollisionEnabled` _barrier "NoCollision")
  (`PrimitiveComponent.SetMaterial` _barrier 0 "/Game/Dynamic/Terrain/MI_Barrier_Green.MI_Barrier_Green"))

(fn `UserConstructionScript`)
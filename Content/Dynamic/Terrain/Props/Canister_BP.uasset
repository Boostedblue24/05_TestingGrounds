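; Canister prop for the infinite terrain that varies its look between clean and dirty variants.
; On BeginPlay it reads the IsClean flag from InfiniteTerrainGameMode, and does nothing if the cast to that game mode fails.
; The flag selects a helper that sets the static mesh's first material slot to one of three random entries from CleanMats or DirtyMats.
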(event `self.ReceiveBeginPlay`
  (bind _asinfinite_terrain_game_mode (cast `/Game/Dynamic/InfiniteTerrainGameMode` (`GameplayStatics.GetGameMode`)))
  (bind _output_get (set `self.IsClean` (`/Game/Dynamic/InfiniteTerrainGameMode.IsClean` _asinfinite_terrain_game_mode)))
  (if _output_get
    (`self.SetRandCleanMat`)
    (else
      (`self.SetRandDirtyMat`))))

(fn `SetRandCleanMat`
  (`PrimitiveComponent.SetMaterial` (`self.StaticMesh`) 0 (`|GetArrayItem` (`self.CleanMats`) (`KismetMathLibrary.RandomInteger` 3))))

(fn `SetRandDirtyMat`
  (`PrimitiveComponent.SetMaterial` (`self.StaticMesh`) 0 (`|GetArrayItem` (`self.DirtyMats`) (`KismetMathLibrary.RandomInteger` 3))))

(fn `UserConstructionScript`)
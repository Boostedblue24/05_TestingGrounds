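; Shipping container prop for the infinite terrain, randomized when play begins.
; On BeginPlay it swings each door to a random yaw of up to 90 degrees, in opposite directions.
; It then reads IsClean from InfiniteTerrainGameMode to pick a random clean or dirty material, applying the same one to the body and both doors.
; The bIsClean function is an unused stub that always returns false.
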(event `self.ReceiveBeginPlay`
  (`SceneComponent.K2_AddLocalRotation` (`self.LeftDoor`) (`KismetMathLibrary.MakeRotator` 0.0 0.0 (`KismetMathLibrary.RandomFloatInRange` 0.0 90.0)) false false)
  (`SceneComponent.K2_AddLocalRotation` (`self.RightDoor`) (`KismetMathLibrary.MakeRotator` 0.0 0.0 (`KismetMathLibrary.RandomFloatInRange` -90.0)) false false)
  (bind _asinfinite_terrain_game_mode (cast `/Game/Dynamic/InfiniteTerrainGameMode` (`GameplayStatics.GetGameMode`)))
  (bind _output_get (set `self.IsClean` (`/Game/Dynamic/InfiniteTerrainGameMode.IsClean` _asinfinite_terrain_game_mode)))
  (if _output_get
    (`self.SetRandCleanMat`)
    (else
      (`self.SetRandDirtyMat`))))

(fn `bIsClean`
  (params (CleanBool :type Boolean))
  (returns (CleanDirty :type Boolean))
  (return false))

(fn `SetRandCleanMat`
  (bind _output_get (set `self.CleanMatToSet` (`|GetArrayItem` (`self.CleanMats`) (`KismetMathLibrary.RandomInteger` 3))))
  (`|ExecutionSequence`
    (:`then_0`
      (`PrimitiveComponent.SetMaterial` (`self.Container`) 0 _output_get))
    (:`then_1`
      (`PrimitiveComponent.SetMaterial` (`self.LeftDoor`) 0 _output_get))
    (:`then_2`
      (`PrimitiveComponent.SetMaterial` (`self.RightDoor`) 0 _output_get))))

(fn `SetRandDirtyMat`
  (bind _output_get (set `self.DirtyMatToSet` (`|GetArrayItem` (`self.DirtyMats`) (`KismetMathLibrary.RandomInteger` 3))))
  (`|ExecutionSequence`
    (:`then_0`
      (`PrimitiveComponent.SetMaterial` (`self.Container`) 0 _output_get))
    (:`then_1`
      (`PrimitiveComponent.SetMaterial` (`self.LeftDoor`) 0 _output_get))
    (:`then_2`
      (`PrimitiveComponent.SetMaterial` (`self.RightDoor`) 0 _output_get))))

(fn `UserConstructionScript`)
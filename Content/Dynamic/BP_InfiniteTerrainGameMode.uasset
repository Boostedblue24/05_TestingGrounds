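; Game mode for an infinite-terrain game that chains procedurally placed tiles and keeps score of tiles passed.
; BeginPlay fills a navmesh bounds volume pool, then spawns the initial run of tiles.
; SpawnTile places each Tile_BP at the previous tile's attach point and hands it the shared pool.
; TilePassed increments the score; the random IsClean flag is unused here, and bIsClean always returns false.
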(event `self.ReceiveBeginPlay`
  (`self.PopulateBoundsVolumePool`)
  (for _ (range 4)
    (`self.SpawnTile`)))

(fn `bIsClean`
  (params (CleanBool :type Boolean))
  (returns (CleanDirty :type Boolean))
  (return false))

(fn `GetScore`
  (returns (Score :type Integer))
  (return (`self.Score`)))

(fn `SpawnTile`
  (set `self.IsClean` (`KismetMathLibrary.RandomBool`))
  (bind _returnvalue (`|SpawnActorFromClass` "/Game/Dynamic/Terrain/Tile_BP.Tile_BP_C" (`self.NextTileTransform`) "Undefined" "OverrideRootScale" null null))
  (`Tile.SetPool` _returnvalue (`self.NavmeshBoundsVolumePool`))
  (bind _attachtransform (`/Game/Dynamic/Terrain/Tile_BP.GetAttachLocation` _returnvalue))
  (set `self.NextTileTransform` _attachtransform))

(fn `TilePassed`
  (`/Engine/EditorBlueprintResources/StandardMacros.IncrementInt` (`self.Score`)))

(fn `UserConstructionScript`)